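; AutoMortar_BP is an auto mortar actor built from tank parts, with a barrel, turret, aiming component and health bar widget.
; On BeginPlay it initialises TankAiming with its barrel and turret, then sets up the health bar.
; The setup casts the widget's user object to HealthBar, assigns itself as that bar's Tank and prints its current health percent.
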(event EventBeginPlay
  (Class|TankAimingComponent|Initialise (Variables|Default|GetTankAiming) (Variables|Default|GetTankBarrel) (Variables|Default|GetTankTurret))
  (CallFunction|InitialiseHealthBar))

(fn ConstructionScript)

(fn InitialiseHealthBar
  (bind _self self)
  (bind _ashealth_bar (Utilities|Casting|CastToHealthBar (UserInterface|GetUserWidgetObject (Variables|Default|GetWidget))))
  (Variables|/Game/UI/HealthBar.HealthBar_C|SetTank _ashealth_bar _self)
  (Development|PrintString (Utilities|String|ToString(Float) (Class|Tank|GetHealthPercent _self))))